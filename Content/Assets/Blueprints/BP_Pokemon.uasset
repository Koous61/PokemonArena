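; Pokemon actor that shows its name, avatar and health in a widget and can be propelled forward by its current owner.
; BeginPlay initializes the UMG_PokemonInfo widget from max health and binds the health-change event to keep it updated.
; While UseFire is set, Tick sweeps the actor along the owner's forward vector by a fixed per-frame step, independent of delta time, until the Fire countdown expires and clears the owner.
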(event `self.ReceiveBeginPlay`
  (add `self.OnChangeHealth` (delegate `UpdateHealth`))
  (bind _asumg_pokemon_info (cast `/Game/Assets/Blueprints/UMG_PokemonInfo` (`WidgetComponent.GetWidget` (`self.Widget`))))
  (bind _returnvalue (`self.GetMaxHealth`))
  (`/Game/Assets/Blueprints/UMG_PokemonInfo.Init` _asumg_pokemon_info (`KismetTextLibrary.Conv_IntToText` _returnvalue) (`KismetTextLibrary.Conv_StringToText` (`self.Name`)) (`self.Avatar`) self)
  (set `self.PokemonInfo` _asumg_pokemon_info))

(event `UpdateHealth` :!signature `self.OnChangeHealth`
  (params (Health :type Integer))
  (`/Game/Assets/Blueprints/UMG_PokemonInfo.UpdateHealth` (`self.PokemonInfo`) (`KismetTextLibrary.Conv_IntToText` Health)))

(event `self.ReceiveTick`
  (params (DeltaSeconds :type "Float (single-precision)"))
  (if (`self.bUseFire`)
    (bind _output_get (set `self.Fire` (- (`self.Fire`) DeltaSeconds)))
    (if (> _output_get 0.0)
      (`self.K2_SetActorLocation` (+ (`self.K2_GetActorLocation`) (* (`self.GetActorForwardVector` (`self.CurrentOwner`)) 2.0)) true)
      (else
        (set `self.bUseFire` false)
        (set `self.Fire` 2.0)
        (set `self.CurrentOwner` null)))))

(fn `UserConstructionScript`)
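; BP_PokemonManager spawns and tracks the level's Pokemon actors.
; On BeginPlay it gathers all TargetPoints and spawns a BP_Pokemon at each until the index exceeds CountPokemon, storing each transform as that Pokemon's SpawnLocation.
; The Respawn input runs SpawnOne, which spawns nothing itself but calls Died on a randomly indexed Pokemon.
; The random range includes the array length, so it can pick an invalid index.
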(event `InputAction|Respawn`
  (params (Key :type "Key Structure"))
  (:`Pressed`
    (`self.SpawnOne`)))

(event `self.ReceiveBeginPlay`
  (bind _outactors (`GameplayStatics.GetAllActorsOfClass` "/Script/Engine.TargetPoint"))
  (set `self.TargetPoint` _outactors)
  (`self.SpawnAll`))

(event `SpawnAll`
  (for (_array_element _array_index) (`self.TargetPoint`)
    (if (<= _array_index (`self.CountPokemon`))
      (bind _returnvalue (`self.GetTransform` _array_element))
      (bind _returnvalue_2 (`|SpawnActorFromClass` "/Game/Assets/Blueprints/BP_Pokemon.BP_Pokemon_C" _returnvalue "Undefined" "OverrideRootScale" null null))
      (set `Pokemon.SpawnLocation` _returnvalue _returnvalue_2)
      (`KismetArrayLibrary.Array_Add` (`self.Pokemons`) _returnvalue_2)
      (else
        (break)))))

(event `SpawnOne`
  (bind _pokemons (`self.Pokemons`))
  (bind _asbp_pokemon (cast `/Game/Assets/Blueprints/BP_Pokemon` (`|GetArrayItem` _pokemons (`KismetMathLibrary.RandomIntegerInRange` 0 (`KismetArrayLibrary.Array_Length` _pokemons)))))
  (`Pokemon.Died` _asbp_pokemon))

(fn `UserConstructionScript`)